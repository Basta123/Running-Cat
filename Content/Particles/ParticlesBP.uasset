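; ParticlesBP is a configurable actor that plays short particle bursts when its box triggers are overlapped.
; When AddCollisions is set, the construction script loops over an index range, adding box and particle component pairs for a base set (index 0) and a Char set (index 1).
; Transforms and templates come from variables.
; Each box's begin overlap activates its particle system, and a brief timer deactivates it, without filtering the overlapping actor.
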(event OnComponentBeginOverlap(BoxCollision)
  (params (OverlappedComponent :type Primitive%20Component%20Object%20Reference) (OtherActor :type Actor%20Object%20Reference) (OtherComp :type Primitive%20Component%20Object%20Reference) (OtherBodyIndex :type Integer) (bFromSweep :type Boolean) (SweepResult :type Hit%20Result%20Structure%20%28by%20ref%29))
  (Components|Activation|Activate (Variables|Default|GetParticleSystem%20%20) false)
  (Utilities|Time|SetTimerbyEvent (delegate Custom|CustomEvent_0) 0.2))

(event OnComponentBeginOverlap(BoxCollisionchar)
  (params (OverlappedComponent :type Primitive%20Component%20Object%20Reference) (OtherActor :type Actor%20Object%20Reference) (OtherComp :type Primitive%20Component%20Object%20Reference) (OtherBodyIndex :type Integer) (bFromSweep :type Boolean) (SweepResult :type Hit%20Result%20Structure%20%28by%20ref%29))
  (Components|Activation|Activate (Variables|Default|GetParticleSystem%20char) false)
  (Utilities|Time|SetTimerbyEvent (delegate Custom|CustomEsent) 0.2))

(event Custom|CustomEsent
  (Components|Activation|Deactivate (Variables|Default|GetParticleSystem%20char)))

(event Custom|CustomEvent_0
  (Components|Activation|Deactivate (Variables|Default|GetParticleSystem%20%20)))

(fn ConstructionScript
  (if (Variables|Default|Getadd%20collisions%20?)
    (for _index (range (Variables|Default|GetFirst%20index%20collision) (Variables|Default|GetLast%20index%20collision))
      (if (== _index 0)
        (bind _returnvalue (AddComponent|AddBoxComponent false))
        (Variables|Default|SetBox%20Collision _returnvalue)
        (Transformation|SetRelativeLocation (Variables|Default|GetBox%20Collision) (Variables|Default|GetLocation%20Box%20Collision) false false)
        (Transformation|SetRelativeScale3D (Variables|Default|GetBox%20Collision) (Variables|Default|GetScale%20Box%20Collision))
        (bind _returnvalue_2 (AddComponent|AddParticleSystemComponent false))
        (Variables|Default|SetParticleSystem%20%20 _returnvalue_2)
        (Transformation|SetRelativeLocation (Variables|Default|GetParticleSystem%20%20) (Variables|Default|GetLocation%20Particle) false false)
        (Effects|Components|ParticleSystem|SetTemplate (Variables|Default|GetParticleSystem%20%20) (Variables|Default|Getparticle))
        (elif (== _index 1)
          (bind _returnvalue_3 (AddComponent|AddBoxComponent false))
          (Variables|Default|SetBox%20Collision%20char _returnvalue_3)
          (Transformation|SetRelativeLocation (Variables|Default|GetBox%20Collision%20char) (Variables|Default|GetLocation%20Box%20Collision%20char) false false)
          (Transformation|SetRelativeScale3D (Variables|Default|GetBox%20Collision%20char) (Variables|Default|GetScale%20Box%20Collision%20char))
          (bind _returnvalue_4 (AddComponent|AddParticleSystemComponent false))
          (Variables|Default|SetParticleSystem%20char _returnvalue_4)
          (Transformation|SetRelativeLocation (Variables|Default|GetParticleSystem%20char) (Variables|Default|GetLocation%20Particle%20char) false false)
          (Effects|Components|ParticleSystem|SetTemplate (Variables|Default|GetParticleSystem%20char) (Variables|Default|Getparticle%20char)))))))