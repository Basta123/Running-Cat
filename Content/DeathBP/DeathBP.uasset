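; DeathBP is an actor that adjusts the player character's capsule during bottom and side deaths.
; It registers with the game instance and game mode, then after a short delay caches the location-specific character's capsule.
; Tick reads externally set flags: bottom death resizes the capsule and conditionally calls Mychar1 for a shake.
; Side death caps capsule height at FirstZ, disabling Tick once it falls below.
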(event Custom|CustomEvent_0
  (bind _mygm (Variables|Default|GetMyGM))
  (bind _mychar3 (Variables|/Game/MyCharacterOther/MyGameMode.MyGameMode_C|Getmychar3 _mygm))
  (bind _mychar1 (Variables|/Game/MyCharacterOther/MyGameMode.MyGameMode_C|Getmychar1 _mygm))
  (switch int (Variables|/Game/Save/MyGameInstance.MyGameInstance_C|Getlocation%20game%20instance (Variables|/Game/MyCharacterOther/MyGameMode.MyGameMode_C|GetMyGI (Variables|Default|GetMyGM)))
    (:1
      (Variables|/Game/MyCharacterOther/Character1/Character1.Character1_C|SetDeathBP _mychar1 self)
      (Variables|Default|SetCapsule%20Component (Variables|/Script/Engine.Character|GetCapsuleComponent _mychar1)))
    (:2
      (Variables|/Game/MyCharacterOther/Character3/Character3.Character3_C|SetDeathBP _mychar3 (Variables|/Game/MyCharacterOther/Character3/Character3.Character3_C|GetDeathBP _mychar3) :!label _label)
      (Variables|Default|SetCapsule%20Component (Variables|/Script/Engine.Character|GetCapsuleComponent _mychar3)))
    (:3
      (goto _label))))

(event EventBeginPlay
  (bind _asmy_game_instance (Utilities|Casting|CastToMyGameInstance (Game|GetGameInstance)))
  (bind _output_get (Variables|Default|SetMyGI _asmy_game_instance))
  (Variables|/Game/Save/MyGameInstance.MyGameInstance_C|SetDeathBP _output_get self)
  (bind _asmy_game_mode (Utilities|Casting|CastToMyGameMode (Game|GetGameMode)))
  (bind _output_get_2 (Variables|Default|SetMyGM _asmy_game_mode))
  (Variables|/Game/MyCharacterOther/MyGameMode.MyGameMode_C|SetDeathBP _output_get_2 self)
  (Utilities|Time|SetTimerbyEvent (delegate Custom|CustomEvent_0) 0.5))

(event EventTick
  (params (DeltaSeconds :type Float%20%28single-precision%29))
  (bind _capsule_component (Variables|Default|GetCapsule%20Component))
  (bind _mygm (Variables|Default|GetMyGM))
  (bind _capsule_component_2 (Variables|Default|GetCapsule%20Component))
  (bind _returnvalue (Transformation|GetWorldLocation _capsule_component))
  (bind _mychar1 (Variables|/Game/MyCharacterOther/MyGameMode.MyGameMode_C|Getmychar1 _mygm))
  (bind (_x _y _z) (Math|Vector|BreakVector _returnvalue))
  (if (Variables|Default|GetDeath%20Bottom%20Work)
    (if (not (Variables|Default|GetDeath%20Bottom%20can%20jump))
      (Components|Capsule|SetCapsuleRadius _capsule_component_2 7e+01 true)
      (Components|Capsule|SetCapsuleHalfHeight _capsule_component_2 7e+01 true)
      (Variables|Default|SetDeath%20Bottom%20can%20jump false)
      (Actor|Tick|SetActorTickEnabled false)
      ;[1 1 1] for shake
      (if (Variables|/Game/MyCharacterOther/Character1/Character1.Character1_C|GetDoes%20call%20from%20DeathBP%20? _mychar1)
        (Variables|/Game/MyCharacterOther/Character1/Character1.Character1_C|SetDoes%20call%20from%20DeathBP%20? _mychar1 true)
        (Default|CallfromDeathBP _mychar1)))
    (elif (Variables|Default|GetDeath%20Side%20Work)
      (if (> (Variables|Default|GetFirst%20Z) _z)
        (Actor|Tick|SetActorTickEnabled false)
        (else
          (Transformation|SetWorldLocation (Variables|Default|GetCapsule%20Component) (Math|Vector|MakeVector _x _y (Variables|Default|GetFirst%20Z)) false false))))))

(fn ConstructionScript)