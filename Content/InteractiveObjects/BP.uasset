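; Actor that flies continuously through the level, wandering between TargetPoints whose sprite component is tagged "Enemy".
; BeginPlay gathers those points, then picks a random one immediately and retries on a looping timer.
; An IfRepeat check is meant to avoid repeats, but the check, selection and stored index each use separate random rolls.
; Tick moves it forward at a fixed per-frame step while RInterpTo gradually turns it toward the current target.
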(event Custom|CustomEvent_0
  (bind _target_array (Variables|Default|GetTarget%20Array))
  (bind _returnvalue (Utilities|Array|LastIndex _target_array))
  (bind _returnvalue_2 (Math|Random|RandomIntegerinRange 0 _returnvalue))
  (if (not (== (Variables|Default|GetIf%20repeat) _returnvalue_2))
    (Variables|Default|SetCurrentTarget (Utilities|Array|Get(acopy) _target_array _returnvalue_2))
    (Variables|Default|SetIf%20repeat _returnvalue_2)))

(event EventBeginPlay
  (bind _target_array (Variables|Default|GetTarget%20Array))
  (bind _returnvalue (Utilities|Array|LastIndex _target_array))
  (bind _returnvalue_2 (Math|Random|RandomIntegerinRange 0 _returnvalue))
  (bind _outactors (Actor|GetAllActorsOfClass "/Script/Engine.TargetPoint"))
  (for _array_element _outactors
    (if (Components|ComponentHasTag (Variables|/Script/Engine.TargetPoint|GetSpriteComponent _array_element) "Enemy")
      (Utilities|Array|Add (Variables|Default|GetTarget%20Array) _array_element)))
  (Utilities|FlowControl|Sequence
    (:then_0
      (Utilities|Time|SetTimerbyEvent (delegate Custom|CustomEvent_0) 4.0 true))
    (:then_1
      (if (not (== (Variables|Default|GetIf%20repeat) _returnvalue_2))
        (Variables|Default|SetCurrentTarget (Utilities|Array|Get(acopy) _target_array _returnvalue_2))
        (Variables|Default|SetIf%20repeat _returnvalue_2)))))

(event EventTick
  (params (DeltaSeconds :type Float%20%28single-precision%29))
  (Transformation|SetActorLocationAndRotation (+ (Transformation|GetActorLocation) (* (Transformation|GetActorForwardVector) 10)) (Math|Interpolation|RInterpTo (Transformation|GetActorRotation) (Math|Rotator|FindLookatRotation (Transformation|GetActorLocation) (Transformation|GetActorLocation (Variables|Default|GetCurrentTarget))) (Utilities|Time|GetWorldDeltaSeconds) 1.2)))

(fn ConstructionScript)