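; Dog actor that runs a scripted dash along world X when it spawns, choosing its behavior from a flag on MyGameMode.
; With DogBeginPlayWorkOrNot set, it slides 3000 units over two seconds, then destroys itself and clears the flag.
; Otherwise, a DoOnce moves it 1750 units over the same time, then sets the game mode's Barks flag.
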(event EventBeginPlay
  (bind _defaultsceneroot (Variables|Default|GetDefaultSceneRoot))
  (bind _returnvalue (Transformation|GetWorldLocation _defaultsceneroot))
  (bind (_x _y _z) (Math|Vector|BreakVector _returnvalue))
  (bind (_x_2 _y_2 _z_2) (Math|Vector|BreakVector _returnvalue))
  (bind _asmy_game_mode (Utilities|Casting|CastToMyGameMode (Game|GetGameMode)))
  (if (Variables|/Game/MyCharacterOther/MyGameMode.MyGameMode_C|GetDog%20Begin%20play%20work%20or%20not _asmy_game_mode)
    (Components|MoveComponentTo _defaultsceneroot (Math|Vector|MakeVector (+ _x_2 3e+03) _y_2 _z_2) "0, 0, 0" false false 2.0)
    (Actor|DestroyActor)
    (bind _asmy_game_mode_2 (Utilities|Casting|CastToMyGameMode (Game|GetGameMode)))
    (Variables|/Game/MyCharacterOther/MyGameMode.MyGameMode_C|SetDog%20Begin%20play%20work%20or%20not _asmy_game_mode_2 false)
    (else
      (Utilities|FlowControl|DoOnce false
        (:Completed
          (Components|MoveComponentTo _defaultsceneroot (Math|Vector|MakeVector (+ _x 1.75e+03) _y _z) "0,0.000000,0.000000" false false 2.0)
          (bind _asmy_game_mode_3 (Utilities|Casting|CastToMyGameMode (Game|GetGameMode)))
          (Variables|/Game/MyCharacterOther/MyGameMode.MyGameMode_C|Setbarks _asmy_game_mode_3 true))))))

(fn ConstructionScript)